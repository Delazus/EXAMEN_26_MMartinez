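; BP_Door is a two-panel door Blueprint, opened or closed through the Open_Door event's boolean.
; The event plays or reverses a Timeline, whose updates lerp the right panel's relative location toward an X offset.
; The left panel's lerp drives relative scale instead of location.
; Both lerp alphas are fixed at zero, and the code capturing initial panel positions never runs, so the panels do not animate.
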(event `Open_Door`
  (params (Open :type Boolean))
  (if Open
    (`Timeline|Timeline` :!label _label
      (:`Update`
        (`SceneComponent.K2_SetRelativeLocation` (`self.Right_Door`) (`KismetMathLibrary.VLerp` (`self.Inist_Pos_DoorRight`) (+ (`self.Inist_Pos_DoorRight`) (110.0 0.0 0.0))) false false)
        (`SceneComponent.SetRelativeScale3D` (`self.Left_Door`) (`KismetMathLibrary.VLerp` (`self.Inist_Pos_DoorLeft`) (+ (`self.Inist_Pos_DoorLeft`) (-110.0 0.0 0.0))))))
    (else
      (goto _label :!via `Reverse`))))

(fn `UserConstructionScript`)