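; BP_FloorButton is an interactive hieroglyph floor button that toggles on the E key and signals state changes through the FloorButtonChangeState dispatcher.
; Box overlap sets Range on BP_ThirdPersonCharacter and enables or disables the button's input.
; E requires PlayerIsInside and Keys, then flips BtnActive, swaps the emissive material and fires the dispatcher.
; The nodes that set PlayerIsInside are disconnected, so this graph never updates that gate.
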(event `self.ReceiveBeginPlay`
  (`PrimitiveComponent.SetMaterial` (`self.SM_hieroglyph_007`) 0 "/Game/00_Examen_UNIR/M_Emission_Off.M_Emission_Off"))

(event `CallOpenEvent`
  (`self.FloorButtonChangeState`))

(event `self.Box.OnComponentBeginOverlap`
  (params (OverlappedComponent :type "PrimitiveComponent Object Reference") (OtherActor :type "Actor Object Reference") (OtherComp :type "PrimitiveComponent Object Reference") (OtherBodyIndex :type Integer) (bFromSweep :type Boolean) (SweepResult :type "HitResult Structure (by ref)"))
  (bind _asbp_third_person_character (cast `/Game/ThirdPerson/Blueprints/BP_ThirdPersonCharacter` OtherActor))
  (set `/Game/ThirdPerson/Blueprints/BP_ThirdPersonCharacter.Range` true _asbp_third_person_character)
  (`self.EnableInput` (`GameplayStatics.GetPlayerController` 0)))

(event `self.Box.OnComponentEndOverlap`
  (params (OverlappedComponent :type "PrimitiveComponent Object Reference") (OtherActor :type "Actor Object Reference") (OtherComp :type "PrimitiveComponent Object Reference") (OtherBodyIndex :type Integer))
  (bind _asbp_third_person_character (cast `/Game/ThirdPerson/Blueprints/BP_ThirdPersonCharacter` OtherActor))
  (set `/Game/ThirdPerson/Blueprints/BP_ThirdPersonCharacter.Range` false _asbp_third_person_character)
  (`self.DisableInput` (`GameplayStatics.GetPlayerController` 0)))

(event `Key|E`
  (params (Key :type "Key Structure"))
  (:`Pressed`
    (if (and (`self.PlayerIsInside`) (`self.Keys`))
      (bind _output_get (set `self.BtnActive` (not (`self.BtnActive`))))
      (if _output_get
        (`PrimitiveComponent.SetMaterial` (`self.SM_hieroglyph_007`) 0 "/Game/00_Examen_UNIR/M_Emission_On.M_Emission_On")
        (`self.CallOpenEvent`)
        (else
          (`PrimitiveComponent.SetMaterial` (`self.SM_hieroglyph_007`) 0 "/Game/00_Examen_UNIR/M_Emission_Off.M_Emission_Off")
          (`self.CallOpenEvent`))))))

(fn `UserConstructionScript`)